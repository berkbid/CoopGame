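; Behavior tree service that picks the AI pawn's target: the nearest living, non-friendly actor known through sight perception.
; Each AI tick it resets the best target, then scans the pawn's known sight-perceived actors, keeping those with a health component above zero that fail the friendly check.
; The closest by distance is written to the blackboard key, or None when none qualifies.
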(event EventReceiveTickAI
  (params (OwnerController :type AI%20Controller%20Object%20Reference) (ControlledPawn :type Pawn%20Object%20Reference) (DeltaSeconds :type Float%20%28single-precision%29))
  ;[1 1 1] Reset everytime we run this service
  (Variables|Default|SetBestTargetActor 0)
  (Variables|Default|SetNearestTargetDistance 1e+06)
  (for _array_element (Class|AIPerceptionComponent|GetKnownPerceivedActors (Actor|GetComponentbyClass ControlledPawn "/Script/AIModule.AIPerceptionComponent") "/Script/AIModule.AISense_Sight")
    (Utilities|IsValid (Actor|GetComponentbyClass _array_element "/Script/CoopGame.SHealthComponent")
      (:Is%20Valid
        (if (and (not (Class|SHealthComponent|IsFriendly _array_element ControlledPawn)) (> (Variables|/Script/CoopGame.SHealthComponent|GetHealth (Actor|GetComponentbyClass _array_element "/Script/CoopGame.SHealthComponent")) 0.0))
          (if (< (Transformation|GetDistanceTo ControlledPawn _array_element) (Variables|Default|GetNearestTargetDistance))
            (Variables|Default|SetNearestTargetDistance (Transformation|GetDistanceTo ControlledPawn _array_element))
            (Variables|Default|SetBestTargetActor _array_element))))))
  ;[1 1 1] After Looping, Assign Best Target Actor
  (Class|BTFunctionLibrary|SetBlackboardValueasObject (Variables|Default|GetBlackboardKey) (Variables|Default|GetBestTargetActor)))